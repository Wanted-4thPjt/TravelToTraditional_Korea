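; BP_CarriageStopPoint is an interactable carriage stop that, as an unfinished prototype, moves the interacting player to a hard-coded location.
; On BeginPlay it binds the Interactable's interaction request (noted as Net Multicast) and state change (noted as client-only).
; The request handler looks up BP_CarriageVehicle without using it, sets the player's location and prints a debug string.
; The state-change handler switches on the new state but does nothing.
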(event Custom|onRequestInteraction_Event
  (params (player :type Pawn%20Object%20Reference))
  (bind _returnvalue (Actor|GetActorOfClass "/Game/YKD/BluePrint/Carriage/BP_CarriageVehicle.BP_CarriageVehicle_C"))
  (Transformation|SetActorLocation player "-100.000000,-100.000000,0.000000" false false)
  (Development|PrintString "Hello"))

(event Custom|CustomEvent_0
  (params (playerController :type Player%20Controller%20Object%20Reference) (newInteractableState :type EInteractableState%20Enum%20%28by%20ref%29 :default "Default"))
  (switch Utilities|FlowControl|Switch|SwitchonEInteractableState newInteractableState))

(event EventBeginPlay
  (bind _interactable (Variables|Default|GetInteractable))
  (Utilities|FlowControl|Sequence
    (:then_0
      (EventDispatchers|AssignOnRequestInteraction _interactable (delegate Custom|onRequestInteraction_Event)) ; Net Multicast 호출
    )
    (:then_1
      (EventDispatchers|BindEventtoOnChangeState _interactable (delegate Custom|CustomEvent_0)) ; Client 전용
    )))

(fn ConstructionScript)