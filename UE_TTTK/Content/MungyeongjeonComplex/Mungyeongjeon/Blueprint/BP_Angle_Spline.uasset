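; Spline builder actor that lays blocking mesh segments along a spline in the construction script, with optional meshes at points.
; Each interval between points gets a segment count from MeshLength, with lengths stretched to fit and halved if too long.
; Segment tangents are sampled slightly past each boundary and clamped to segment length.
; Index lists swap in alternate segment or point meshes, and point meshes appear only on CurveClamped points.
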(event EventBeginPlay)

(event Collision|EventActorBeginOverlap
  (params (OtherActor :type Actor%20Object%20Reference)))

(event EventTick
  (params (DeltaSeconds :type Float%20%28single-precision%29)))

(fn ConstructionScript
  (bind _spline (Variables|Default|GetSpline))
  (bind _spline_2 (Variables|Default|GetSpline))
  ;[1 1 1] 포인트 인덱스 확인
  (for _index (range 0 (- (Spline|GetNumberOfSplinePoints (Variables|Default|GetSpline)) 1))
    (Variables|Default|SetCurrent%20Spline%20Index _index)
    (Utilities|FlowControl|Sequence
      (:then_0
        ;[1 1 1] 포인트와 포인트사이의 길이 계산 및 배치 가능한 메시 개수 설정
        (Variables|Default|SetCurrnet%20Spline%20Distance (Spline|GetDistanceAlongSplineatSplinePoint (Variables|Default|GetSpline) (Variables|Default|GetCurrent%20Spline%20Index)))
        (bind _output_get (Variables|Default|SetCurrnet%20Spline%20Lenght (- (Spline|GetDistanceAlongSplineatSplinePoint (Variables|Default|GetSpline) (+ (Variables|Default|GetCurrent%20Spline%20Index) 1)) (Spline|GetDistanceAlongSplineatSplinePoint (Variables|Default|GetSpline) (Variables|Default|GetCurrent%20Spline%20Index)))))
        (Variables|Default|SetCurrnet%20Spline%20Num%20Mesh (/ _output_get (Variables|Default|GetMeshLength)))
        ;[1 1 1] 배치할 메시 길이 설정
        (bind _output_get_2 (Variables|Default|SetElongated%20Mesh%20Length (/ (Variables|Default|GetCurrnet%20Spline%20Lenght) (Variables|Default|GetCurrnet%20Spline%20Num%20Mesh))))
        (if (< _output_get_2 (* (Variables|Default|GetMeshLength) 1.5))
          _
          (else
            (Variables|Default|SetElongated%20Mesh%20Length (/ (Variables|Default|GetElongated%20Mesh%20Length) 2.0))
            (Variables|Default|SetCurrnet%20Spline%20Num%20Mesh (* (Variables|Default|GetCurrnet%20Spline%20Num%20Mesh) 2))))
        (for _index_2 (range 0 (- (Variables|Default|GetCurrnet%20Spline%20Num%20Mesh) 1))
          (Math|Integer|IncrementInt (Variables|Default|GetSegment%20Index)
            (:%20%20
              ;[1 1 1] 메시추가
              (bind _returnvalue (AddComponent|AddSplineMeshComponent false))
              (Collision|SetCollisionEnabled _returnvalue "QueryAndPhysics")
              (Collision|SetCollisionProfileName _returnvalue "BlockAll" true :!class /Script/Engine.PrimitiveComponent)
              (bind _output_get_3 (Variables|Default|SetSegment%20SM%20Var _returnvalue))
              (SplineMesh|SetStartandEnd _output_get_3 (Spline|GetLocationatDistanceAlongSpline _spline_2 (+ (* _index_2 (Variables|Default|GetElongated%20Mesh%20Length)) (Variables|Default|GetCurrnet%20Spline%20Distance)) "Local") (Math|Vector|ClampVectorSize (Spline|GetTangentatDistanceAlongSpline _spline_2 (+ (+ (* _index_2 (Variables|Default|GetElongated%20Mesh%20Length)) (Variables|Default|GetCurrnet%20Spline%20Distance)) 1.0) "Local") 1.0 (Variables|Default|GetElongated%20Mesh%20Length)) (Spline|GetLocationatDistanceAlongSpline _spline (+ (* (+ _index_2 1) (Variables|Default|GetElongated%20Mesh%20Length)) (Variables|Default|GetCurrnet%20Spline%20Distance)) "Local") (Math|Vector|ClampVectorSize (Spline|GetTangentatDistanceAlongSpline _spline (+ (+ (* (+ _index_2 1) (Variables|Default|GetElongated%20Mesh%20Length)) (Variables|Default|GetCurrnet%20Spline%20Distance)) 1.0) "Local") 1.0 (Variables|Default|GetElongated%20Mesh%20Length)) true :!class /Script/Engine.SplineMeshComponent)
              (Utilities|FlowControl|Sequence
                (:then_0
                  (if (Utilities|Array|ContainsItem (Variables|Segment|GetChange%20A%20Segment) (Variables|Default|GetSegment%20Index))
                    (Components|StaticMesh|SetStaticMesh (Variables|Default|GetSegment%20SM%20Var) (Utilities|Select :Index (Variables|Segment|GetSelect%20A%20Segment) :Option%200 (Variables|Segment|Get0%20SegmentMesh) :Option%201 (Variables|Segment|Get1%20SegmentMesh) :Option%202 0))
                    (else
                      (Components|StaticMesh|SetStaticMesh (Variables|Default|GetSegment%20SM%20Var) (Variables|Default|GetNew%20Mesh))))))))))
      (:then_1
        (Math|Integer|IncrementInt (Variables|Default|GetPoint%20Index)
          (:%20%20
            (if (Variables|Default|GetCouner%20Mesh%20Use)
              (if (Utilities|Enum|Equal(Enum) (Class|SplineComponent|GetSplinePointType (Variables|Default|GetSpline) (Variables|Default|GetCurrent%20Spline%20Index)) "CurveClamped")
                (bind _returnvalue_2 (AddComponent|AddStaticMeshComponent false (Spline|GetTransformatSplinePoint (Variables|Default|GetSpline) (Variables|Default|GetCurrent%20Spline%20Index) "Local" false)))
                (if (Utilities|Array|ContainsItem (Variables|Point|GetChange%20Point) (Variables|Default|GetPoint%20Index))
                  (Components|StaticMesh|SetStaticMesh _returnvalue_2 (Utilities|Select :Index (Variables|Point|GetSelect%20Point) :Option%200 (Variables|Point|Get0%20Point%20Mesh) :Option%201 (Variables|Point|Get1%20Point%20Mesh)))
                  (else
                    (Components|StaticMesh|SetStaticMesh _returnvalue_2 (Variables|Point|GetPoint%20Mesh))))))))))))